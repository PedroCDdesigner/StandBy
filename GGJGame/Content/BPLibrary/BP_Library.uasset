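; BP_Library is a Blueprint function library with a helper that switches player control to another robot pawn.
; FRobotPossess acts only when the requested robot number differs from the current one and no possession is flagged as active.
; If that robot's RobotEnergy is above zero, player controller 0 possesses it, and the function returns the new robot number and possession flag.
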(fn `F Robot Possess`
  (params (`Robot Pawn` :type "/Game/FirstPersonBP/Blueprints/FirstPersonCharacter Object Reference") (`Robot to Possess` :type Integer) (`Current Robot Number` :type Integer) (isPossessing :type Boolean))
  (returns (`New Current Robot Number` :type Integer) (`New isPossessing` :type Boolean))
  (locals (Local_currentRobotNumber :type Integer :default 1) (Local_isPossessing :type Boolean) (LocalRobotPawn :type "/Game/FirstPersonBP/Blueprints/FirstPersonCharacter Object Reference") (LocalRobotToPossess :type Integer))
  (bind _returnvalue (`GameplayStatics.GetPlayerController` null))
  (set `local.LocalRobotPawn` `Robot Pawn`)
  (bind _output_get (set `local.LocalRobotToPossess` `Robot to Possess`))
  (bind _output_get_2 (set `local.Local_currentRobotNumber` `Current Robot Number`))
  (`/Engine/EditorBlueprintResources/StandardMacros.CompareInt` _output_get _output_get_2
    (:`>`
      _)
    (:`==`
      (return (`local.Local_currentRobotNumber`) (`local.Local_isPossessing`)))
    (:`<`
      _))
  (bind _output_get_3 (set `local.Local_isPossessing` isPossessing))
  (if _output_get_3
    (return (`local.Local_currentRobotNumber`) true)
    (else
      (`/Engine/EditorBlueprintResources/StandardMacros.CompareInt` (`/Game/FirstPersonBP/Blueprints/FirstPersonCharacter.RobotEnergy` (`local.LocalRobotPawn`))
        (:`>`
          (set `local.Local_currentRobotNumber` (`local.LocalRobotToPossess`))
          (cast `PlayerController` _returnvalue)
          (`Controller.Possess` _returnvalue (`local.LocalRobotPawn`))
          (return (`local.Local_currentRobotNumber`) true))))))